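; BP_item is a pickup item whose mesh is set in the Construction Script from a variable.
; Its Pickup event plays a timeline that shrinks the root's world scale to zero.
; A DoOnce on the timeline's update plays the pickup sound once, then destroys the actor after a short delay.
; Box overlap with a BP_Ai only prints a debug message.
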(event `/Game/Pickup/BPI_ITEMS.pickup`
  (`KismetSystemLibrary.PrintString` "Hello")
  (bind (_direction _shrink) (`Timeline|shrink`)
    (:`Update`
      (`SceneComponent.SetWorldScale3D` (`self.DefaultSceneRoot`) (`KismetMathLibrary.Conv_DoubleToVector` (`KismetMathLibrary.Lerp` 1.0 0.0 _shrink)))
      (`/Engine/EditorBlueprintResources/StandardMacros.DoOnce` false
        (:`Completed`
          (`GameplayStatics.PlaySound2D` "/Engine/VREditor/Sounds/UI/Object_PickUp.Object_PickUp" 1.0 1.0 0.0 null null)
          (`KismetSystemLibrary.Delay` 0.4)
          (`self.K2_DestroyActor`))))))

(event `self.Box.OnComponentBeginOverlap`
  (params (OverlappedComponent :type "PrimitiveComponent Object Reference") (OtherActor :type "Actor Object Reference") (OtherComp :type "PrimitiveComponent Object Reference") (OtherBodyIndex :type Integer) (bFromSweep :type Boolean) (SweepResult :type "HitResult Structure (by ref)"))
  (cast `/Game/Ai/BP_Ai` OtherActor)
  (`KismetSystemLibrary.PrintString` "ah shit casper" true true (struct :`G` 0.66 :`B` 1.0 :`A` 1.0) 11.0))

(fn `UserConstructionScript`
  (`StaticMeshComponent.SetStaticMesh` (`self.itemmodel`) (`self.itemodelto`)))