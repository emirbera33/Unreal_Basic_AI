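; BP_Ai is an AI pawn that reacts to seeing the player, with collision logic noted as being for passing through walls.
; The construction script starts ColTest with query and physics collision.
; When PawnSensing sees a pawn tagged "player", it sets the "seeingplayer" Blackboard key to true and disables ColTest collision.
; Nothing in this Blueprint clears the key or restores collision afterward.
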(event `self.ReceiveBeginPlay`)

(event `self.PawnSensing.OnSeePawn`
  (params (Pawn :type "Pawn Object Reference"))
  ;[1 1 1] Duvardan geçme collision
  (if (`self.ActorHasTag` Pawn "player")
    (`BlackboardComponent.SetValueAsBool` (`AIBlueprintHelperLibrary.GetBlackboard` (`AIBlueprintHelperLibrary.GetAIController` self)) "seeingplayer" true)
    (`PrimitiveComponent.SetCollisionEnabled` (`self.col_test`) "NoCollision")))

(fn `UserConstructionScript`
  (`PrimitiveComponent.SetCollisionEnabled` (`self.col_test`) "QueryAndPhysics"))