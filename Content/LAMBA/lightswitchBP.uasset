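; Light switch Blueprint that lets the player toggle linked lights by pressing F while inside its trigger box.
; On BeginPlay it gathers every LightBP actor in the level into an array.
; The box overlap enables or disables player input and opens or closes a gate around the F key.
; A press through the open gate calls ToggleLightsMessage on each light whose LightIndex matches the switch's own.
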(event `self.ReceiveBeginPlay`
  (bind _outactors (`GameplayStatics.GetAllActorsOfClass` "/Game/LAMBA/lightBP.lightBP_C"))
  (for _array_element _outactors
    (`KismetArrayLibrary.Array_Add` (`self.light array`) _array_element)))

(event `Key|F`
  (params (Key :type "Key Structure"))
  (:`Pressed`
    (`/Engine/EditorBlueprintResources/StandardMacros.Gate` true :!label _label
      (:`Exit`
        (for _array_element (`self.light array`)
          (if (== (`/Game/LAMBA/lightBP.light index` _array_element) (`self.light index`))
            (message `/Game/LAMBA/Lightinterface.toggle lights` _array_element)))))))

(event `self.Box.OnComponentBeginOverlap`
  (params (OverlappedComponent :type "PrimitiveComponent Object Reference") (OtherActor :type "Actor Object Reference") (OtherComp :type "PrimitiveComponent Object Reference") (OtherBodyIndex :type Integer) (bFromSweep :type Boolean) (SweepResult :type "HitResult Structure (by ref)"))
  (`self.EnableInput` (`GameplayStatics.GetPlayerController` 0))
  (goto _label :!via `Open`))

(event `self.Box.OnComponentEndOverlap`
  (params (OverlappedComponent :type "PrimitiveComponent Object Reference") (OtherActor :type "Actor Object Reference") (OtherComp :type "PrimitiveComponent Object Reference") (OtherBodyIndex :type Integer))
  (`self.DisableInput` (`GameplayStatics.GetPlayerController` 0))
  (goto _label :!via `Close`))

(fn `UserConstructionScript`)