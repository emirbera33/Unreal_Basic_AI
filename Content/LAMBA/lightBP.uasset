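; Light fixture Blueprint with three spot lights that switch on and off together.
; The ToggleLights event flips the On boolean and applies it as the visibility of all three lights.
; The construction script applies the same On value, so the placed actor shows its initial lit or unlit state.
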(event `/Game/LAMBA/Lightinterface.toggle lights`
  (bind _output_get (set `self.on?` (not (`self.on?`))))
  (`SceneComponent.SetVisibility` (`self.SpotLight2`) _output_get false)
  (`SceneComponent.SetVisibility` (`self.SpotLight1`) _output_get false)
  (`SceneComponent.SetVisibility` (`self.SpotLight`) _output_get false))

(fn `UserConstructionScript`
  (`SceneComponent.SetVisibility` (`self.SpotLight2`) (`self.on?`) false)
  (`SceneComponent.SetVisibility` (`self.SpotLight1`) (`self.on?`) false)
  (`SceneComponent.SetVisibility` (`self.SpotLight`) (`self.on?`) false))