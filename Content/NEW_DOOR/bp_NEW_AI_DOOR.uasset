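; Test-style AI pawn that finds a nearby door at BeginPlay, walks through it, then wanders.
; The search loops over NEW_BPDOOR actors, widening its distance threshold after each miss until one qualifies.
; It moves to the nearer of the door's two reference points, pauses briefly, then crosses to the other.
; RandomRoom then repeatedly moves it to random reachable points with random pauses.
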(event `self.ReceiveBeginPlay`
  (`self.Find Nearest door`))

(event `Find Nearest door`
  ;[1 1 1] AI Kapı arama
  (set `self.searching for door ?` true)
  (bind _outactors (`GameplayStatics.GetAllActorsOfClass` "/Game/NEW_DOOR/NEW_BPDOOR.NEW_BPDOOR_C"))
  (for _array_element _outactors :!label _label
    (if (<= (`self.GetDistanceTo` _array_element) (`self.Distance`))
      (set `self.searching for door ?` false)
      (set `self.Distance` 100.0)
      (set `self.Door ref` _array_element)
      (break)
      (else
        (set `self.Distance` (+ (`self.Distance`) 50.0)))))
  (if (`self.searching for door ?`)
    (goto _label)
    (else
      (`self.go to door open`))))

(event `go to door open`
  (bind _returnvalue (`self.K2_GetActorLocation`))
  (bind _door_ref (`self.Door ref`))
  (bind _returnvalue_2 (`SceneComponent.K2_GetComponentLocation` (`/Game/NEW_DOOR/NEW_BPDOOR.referans2` _door_ref)))
  (bind _returnvalue_3 (`SceneComponent.K2_GetComponentLocation` (`/Game/NEW_DOOR/NEW_BPDOOR.Referans1` _door_ref)))
  ;[1 1 1] Kapıyı bulduktan sonra kapının önü mü arkası mı onu tespit etme
  (if (< (`KismetMathLibrary.VSize` (- _returnvalue _returnvalue_3)) (`KismetMathLibrary.VSize` (- _returnvalue _returnvalue_2)))
    (`|AIMoveTo` self _returnvalue_3 null
      (:`OnSuccess`
        (`KismetSystemLibrary.Delay` 0.2)
        (`|AIMoveTo` self _returnvalue_2 null
          (:`OnSuccess`
            _))))
    (else
      (`|AIMoveTo` self _returnvalue_2 null
        (:`OnSuccess`
          (`KismetSystemLibrary.Delay` 0.2)
          (`|AIMoveTo` self _returnvalue_3 null
            (:`OnSuccess`
              _))))))
  (`self.Random room`))

(event `Random room`
  ;[1 1 1] random hareket
  (`|AIMoveTo` self (`NavigationSystemV1.K2_GetRandomReachablePointInRadius` (`self.K2_GetActorLocation`) 1500.0 null null) null
    (:`OnSuccess`
      (`KismetSystemLibrary.Delay` (`KismetMathLibrary.RandomFloatInRange` 1.0 3.0))
      (`self.Random room`))))

(fn `UserConstructionScript`)